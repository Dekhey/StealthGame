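; Sealed door Blueprint that shows a barred gate mesh (PuertaReja) with a dissolve-capable material.
; The Construction Script assigns the mesh, creates a dynamic instance of MI_DissolveSealed on its first material slot and stores it in DynamicDissolveMaterial.
; The Event Graph holds only disabled default events, so this graph does not drive the dissolve itself.
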(fn `UserConstructionScript`
  (bind _mesh (`self.Mesh`))
  (`StaticMeshComponent.SetStaticMesh` (`self.Mesh`) "/Game/Arte/Modelos3D/PuertaReja/PuertaReja.PuertaReja")
  (bind _returnvalue (`PrimitiveComponent.CreateDynamicMaterialInstance` _mesh 0 "/Game/Arte/Modelos3D/PuertaReja/Texturas/MI_DissolveSealed.MI_DissolveSealed" "None"))
  (bind _output_get (set `self.DynamicDissolveMaterial` _returnvalue))
  (`PrimitiveComponent.SetMaterial` _mesh 0 _output_get))