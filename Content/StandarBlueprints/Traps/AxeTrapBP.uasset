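; AxeTrapBP is a trap actor that swings its mesh, presumably an axe, by rotating it on the pitch axis.
; A timeline drives the rotation and restarts from the start each time it finishes, looping while the trap is active.
; ActivateTrap toggles the Active flag and starts playback when enabled.
; An event track on the timeline checks the flag and stops the swing once deactivated, rather than stopping immediately.
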(event `self.ReceiveBeginPlay`
  (if (`self.bActive`)
    (bind (_direction _rotation) (`Timeline|Timeline` :!label _label)
      (:`Update`
        (`SceneComponent.K2_SetRelativeRotation` (`self.Mesh`) (`KismetMathLibrary.MakeRotator` 0.0 _rotation) false false))
      (:`Finished`
        (goto _label :!via `PlayFromStart`))
      (:`NewTrack_1`
        (if (not (`self.bActive`))
          (goto _label :!via `Stop`))))))

(event `self.ActivateTrap`
  (bind _output_get (set `self.bActive` (not (`self.bActive`))))
  (if _output_get
    (goto _label)))

(fn `UserConstructionScript`)