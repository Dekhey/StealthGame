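; LogTrapBP is a log trap actor that swings or pivots its mesh when the ActivateTrap event fires.
; A timeline's curve drives the mesh's relative pitch each update.
; Timeline event tracks flip a Direction value and, at the finish point, disable the separate Collision component while setting the mesh to query and physics collision.
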(event `self.ActivateTrap`
  ;[1 1 1] Activate trap
  (bind (_direction _logtrapcurve) (`Timeline|Timeline`)
    (:`Update`
      (`SceneComponent.K2_SetRelativeRotation` (`self.Mesh`) (`KismetMathLibrary.MakeRotator` 0.0 _logtrapcurve) false false))
    (:`LogDirection`
      (set `self.direction` (* (`self.direction`) -1)))
    (:`FinishCollision`
      (`PrimitiveComponent.SetCollisionEnabled` (`self.Collision`) "NoCollision")
      (`PrimitiveComponent.SetCollisionEnabled` (`self.Mesh`) "QueryAndPhysics"))))

(fn `UserConstructionScript`)