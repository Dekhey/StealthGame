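; ManaSpringBP is a world actor that boosts the main character's mana regeneration while the character stands inside it.
; On Collision begin overlap it casts the other actor to MainCharacterBP and multiplies its ManaRegSpeed by ManaIncrement.
; On end overlap it divides by the same factor to undo the boost, rather than storing and restoring the original value.
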(event `self.Collision.OnComponentBeginOverlap`
  (params (OverlappedComponent :type "PrimitiveComponent Object Reference") (OtherActor :type "Actor Object Reference") (OtherComp :type "PrimitiveComponent Object Reference") (OtherBodyIndex :type Integer) (bFromSweep :type Boolean) (SweepResult :type "HitResult Structure (by ref)"))
  (bind _asmain_character_bp (cast `/Game/Characters/MainCharacter/MainCharacterBP` OtherActor))
  (set `/Game/Characters/MainCharacter/MainCharacterBP.ManaRegSpeed` (* (`/Game/Characters/MainCharacter/MainCharacterBP.ManaRegSpeed` _asmain_character_bp) (`self.ManaIncrement`)) _asmain_character_bp))

(event `self.Collision.OnComponentEndOverlap`
  (params (OverlappedComponent :type "PrimitiveComponent Object Reference") (OtherActor :type "Actor Object Reference") (OtherComp :type "PrimitiveComponent Object Reference") (OtherBodyIndex :type Integer))
  (bind _asmain_character_bp (cast `/Game/Characters/MainCharacter/MainCharacterBP` OtherActor))
  (set `/Game/Characters/MainCharacter/MainCharacterBP.ManaRegSpeed` (/ (`/Game/Characters/MainCharacter/MainCharacterBP.ManaRegSpeed` _asmain_character_bp) (`self.ManaIncrement`)) _asmain_character_bp))

(fn `UserConstructionScript`)