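; DissolveDoorBP is a grate door that dissolves away and destroys itself when StartDissolve is called.
; Its construction script assigns the mesh and a dynamic instance of MI_Dissolve.
; Overlapping DissolveRadius sets Dissolve on the door and NearDissolveDoor on MainCharacterBP, clearing both on exit, without starting the effect.
; StartDissolve plays a timeline that drives the material's Length parameter, then destroys the actor.
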(event `self.DissolveRadius.OnComponentBeginOverlap`
  (params (OverlappedComponent :type "PrimitiveComponent Object Reference") (OtherActor :type "Actor Object Reference") (OtherComp :type "PrimitiveComponent Object Reference") (OtherBodyIndex :type Integer) (bFromSweep :type Boolean) (SweepResult :type "HitResult Structure (by ref)"))
  ;[1 1 1] Collision
  (bind _asmain_character_bp (cast `/Game/Characters/MainCharacter/MainCharacterBP` OtherActor))
  (set `/Game/Characters/MainCharacter/MainCharacterBP.bNearDissolveDoor` true _asmain_character_bp)
  (set `self.bDissolve` true))

(event `self.DissolveRadius.OnComponentEndOverlap`
  (params (OverlappedComponent :type "PrimitiveComponent Object Reference") (OtherActor :type "Actor Object Reference") (OtherComp :type "PrimitiveComponent Object Reference") (OtherBodyIndex :type Integer))
  ;[1 1 1] Collision
  (bind _asmain_character_bp (cast `/Game/Characters/MainCharacter/MainCharacterBP` OtherActor))
  (set `/Game/Characters/MainCharacter/MainCharacterBP.bNearDissolveDoor` false _asmain_character_bp)
  (set `self.bDissolve` false))

(event `StartDissolve`
  ;[1 1 1] Dissolve Event
  (bind (_direction _dissolvecurvelength) (`Timeline|DissolveDoorTimeline` :!via `PlayFromStart`)
    (:`Update`
      (bind _asmaterial_instance_dynamic (cast `MaterialInstanceDynamic` (`PrimitiveComponent.GetMaterial` (`self.Mesh`) 0))
        (:`then`
          (`MaterialInstanceDynamic.SetScalarParameterValue` _asmaterial_instance_dynamic "Length" _dissolvecurvelength))
        (:`CastFailed`
          (`KismetSystemLibrary.PrintString` "The material in the door isn't dynamic"))))
    (:`Finished`
      (`self.K2_DestroyActor`))))

(fn `UserConstructionScript`
  (bind _mesh (`self.Mesh`))
  (`StaticMeshComponent.SetStaticMesh` (`self.Mesh`) "/Game/Arte/Modelos3D/PuertaReja/PuertaReja.PuertaReja")
  (bind _returnvalue (`PrimitiveComponent.CreateDynamicMaterialInstance` _mesh 0 "/Game/Arte/Modelos3D/PuertaReja/Texturas/MI_Dissolve.MI_Dissolve" "None"))
  (bind _output_get (set `self.DynamicDissolveMaterial` _returnvalue))
  (`PrimitiveComponent.SetMaterial` _mesh 0 _output_get))